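; BP_Enemy is an enemy character that attacks with a weapon and handles its own death.
; On BeginPlay it binds its attack event to the BP_AI controller's attack signature, passing each signal on to the Weapon.
; When its Health reports death, it prints a message, disables movement, plays the death montage, waits out the returned duration, then sets a short lifespan to remove itself.
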(event OnDeath(Health)
  (Development|PrintString (Utilities|String|Append (Utilities|GetDisplayName self) "" "Is Dead"))
  (Pawn|Components|CharacterMovement|DisableMovement (Variables|Character|GetCharacterMovement))
  (bind _returnvalue (Animation|PlayAnimMontage "/Game/External_Content/Animations/UE4_rig/AM_Death.AM_Death" 1.0 "None"))
  (Utilities|FlowControl|Delay _returnvalue)
  (Actor|SetLifeSpan 1.0))

(event Custom|attack
  (Class|ChTWeaponComponent|Attack (Variables|Default|GetWeapon)))

(event EventBeginPlay
  (bind _asbp_ai (Utilities|Casting|CastToBP_AI (Pawn|GetController)))
  (EventDispatchers|BindEventtoAttackSignature _asbp_ai (delegate Custom|attack)))

(event Collision|EventActorBeginOverlap
  (params (OtherActor :type Actor%20Object%20Reference)))

(event EventTick
  (params (DeltaSeconds :type Float%20%28single-precision%29)))

(fn ConstructionScript)