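; Behavior tree task that records how far the AI-controlled pawn is from its target actor.
; On execute, it reads TargetActor from the blackboard and writes the distance between the two actor locations to DistanceToTarget, using hardcoded key names.
; It finishes with the success of the Actor cast, though the distance is written without checking that cast first.
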(event EventReceiveExecuteAI
  (params (OwnerController :type AI%20Controller%20Object%20Reference) (ControlledPawn :type Pawn%20Object%20Reference))
  (bind _returnvalue (Utilities|Name|MakeLiteralName "TargetActor"))
  (bind _returnvalue_2 (AI|GetBlackboard OwnerController))
  (bind _returnvalue_3 (AI|Components|Blackboard|GetValueasObject _returnvalue_2 _returnvalue))
  (bind (_asactor _bsuccess) (Utilities|Casting|CastToActor _returnvalue_3))
  (AI|Components|Blackboard|SetValueasFloat _returnvalue_2 (Utilities|Name|MakeLiteralName "DistanceToTarget") (Math|Vector|Distance(Vector) (Transformation|GetActorLocation ControlledPawn) (Transformation|GetActorLocation _asactor)))
  (AI|BehaviorTree|FinishExecute _bsuccess))