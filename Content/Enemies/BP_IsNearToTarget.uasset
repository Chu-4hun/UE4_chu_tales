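; Behavior tree task that checks how close an AI-controlled enemy pawn is to its target actor.
; On execution it measures the distance from the pawn to the blackboard's TargetActor and writes it to DistanceToTarget.
; It sets IsNearToTarget when that distance is below RequiredDistance, then always finishes successfully.
; Blackboard keys are referenced by hardcoded names, and the target cast has no validity check.
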(event EventReceiveExecuteAI
  (params (OwnerController :type AI%20Controller%20Object%20Reference) (ControlledPawn :type Pawn%20Object%20Reference))
  (bind _returnvalue (Utilities|Name|MakeLiteralName "TargetActor"))
  (bind _returnvalue_2 (Transformation|GetActorLocation ControlledPawn))
  (bind _returnvalue_3 (AI|GetBlackboard OwnerController))
  (bind _returnvalue_4 (AI|Components|Blackboard|GetValueasObject _returnvalue_3 _returnvalue))
  (bind _asactor (Utilities|Casting|CastToActor _returnvalue_4))
  (bind _returnvalue_5 (Transformation|GetActorLocation _asactor))
  (bind _returnvalue_6 (Math|Vector|Distance(Vector) _returnvalue_2 _returnvalue_5))
  (AI|Components|Blackboard|SetValueasFloat _returnvalue_3 (Utilities|Name|MakeLiteralName "DistanceToTarget") _returnvalue_6)
  (AI|Components|Blackboard|SetValueasBool _returnvalue_3 (Utilities|Name|MakeLiteralName "IsNearToTarget") (< _returnvalue_6 (Variables|Default|GetRequiredDistance)))
  (AI|BehaviorTree|FinishExecute true))