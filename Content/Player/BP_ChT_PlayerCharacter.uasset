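; Player character Blueprint that provides a foot-trace helper for IK foot placement.
; IKFootTrace line-traces on Visibility from actor height at a mesh socket's XY down to a given distance below the socket, with one-frame debug drawing.
; A hit returns its location, height relative to the mesh minus IKHipOffset, and a fixed-offset socket position; a miss returns zeros.
; Tick and construction script are empty.
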(event EventTick
  (params (DeltaSeconds :type Float%20%28single-precision%29)))

(fn ConstructionScript)

(fn IKFootTrace
  (params (SocketName :type Name) (Distance :type Float%20%28single-precision%29))
  (bind _mesh (Variables|Character|GetMesh))
  (bind _returnvalue (Transformation|GetSocketLocation _mesh SocketName))
  (bind (_outhit _returnvalue_2) (Collision|LineTraceByChannel (Math|Vector|MakeVector (.x _returnvalue) (.y _returnvalue) (.z (Transformation|GetActorLocation))) (Math|Vector|MakeVector (.x _returnvalue) (.y _returnvalue) (- (.z _returnvalue) Distance)) "TraceTypeQuery1" false 0 "ForOneFrame"))
  (if _returnvalue_2
    (return (.location _outhit) (- (.z (- (.location _outhit) (Transformation|GetWorldLocation (Variables|Character|GetMesh)))) (Variables|Default|GetIK_HipOffset)) (+ (Transformation|GetSocketLocation (Variables|Character|GetMesh) SocketName) "15.000000,200.000000,40.000000"))
    (else
      (return "0, 0, 0" 0.0 "0, 0, 0"))))